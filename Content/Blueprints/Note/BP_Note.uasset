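; BP_Note is a note object that shows a readable image on screen when checked.
; On BeginPlay it applies its NoteMaterial to the Note component.
; NoteCheck creates a WB_Notes widget for the first player controller, passes it WidgetImage and adds it to the viewport.
; NoteClose removes that widget from its parent.
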(event Custom|NoteCheck
  (bind _returnvalue (UserInterface|CreateWidget "/Game/UI/WB_Notes.WB_Notes_C" (Game|GetPlayerController 0)))
  (bind _aswb_notes (Utilities|Casting|CastToWB_Notes _returnvalue))
  (Default|SetNote _aswb_notes (Variables|Default|GetWidgetImage))
  (UserInterface|Viewport|AddtoViewport _returnvalue 0))

(event Custom|NoteClose
  (Widget|RemovefromParent (stale Custom|NoteCheck _returnvalue)))

(event EventBeginPlay
  (Rendering|Material|SetMaterial (Variables|Default|GetNote) 0 (Variables|Default|GetNoteMaterial)))

(fn ConstructionScript)