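; BP_NumberInput is a code-entry puzzle that checks a three-digit number sequence and opens doors when it is correct.
; On BeginPlay it copies the answer array from BP_RandomNumberParent, and each entered number is appended to a display text with a beep.
; After three inputs it compares element by element, either resetting with a fail buzzer or playing a success sound, destroying the Door actors and completing an objective in WB_TabeMenu.
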(event Custom|AddNumberToAnswer
  (bind _input (Variables|Default|GetInput))
  (bind _numberinput (Variables|Default|GetNumberInput))
  (Utilities|Array|Add (Variables|Default|GetInputAnswer) _numberinput)
  (Development|PrintString (Utilities|String|ToString(Integer) _numberinput))
  (Math|Integer|IncrementInt _input
    (:%20%20
      (bind _output_get (Variables|Default|SetInputText (Utilities|String|Append (Variables|Default|GetInputText) (Utilities|String|ToString(Integer) (Variables|Default|GetNumberInput)))))
      (Rendering|Components|TextRender|SetText (Variables|Default|GetAnswer) (Utilities|Text|ToText(String) _output_get))
      (Audio|PlaySound2D "/Game/Audio/one_beep-99630.one_beep-99630" 1.0 1.0 0.0 0 0)
      (if (== _input 3)
        (CallFunction|CheckAnswer)))))

(event Custom|CheckAnswer
  (if (== (Utilities|Array|Length (Variables|Default|GetInputAnswer)) (Utilities|Array|Length (Variables|Default|GetActAnswer)))
    (for (_array_element _array_index) (Variables|Default|GetInputAnswer)
      (Development|PrintString (Utilities|String|ToString(Boolean) (== _array_element (Utilities|Array|Get(acopy) (Variables|Default|GetActAnswer) _array_index))))
      (if (== _array_element (Utilities|Array|Get(acopy) (Variables|Default|GetActAnswer) _array_index))
        (Math|Integer|IncrementInt (Variables|Default|GetAllCorrect))))
    (if (== (Variables|Default|GetAllCorrect) 3)
      (Variables|Default|SetInput 0)
      (Audio|PlaySound2D "/Game/Audio/90s-game-ui-6-185099.90s-game-ui-6-185099" 1.0 1.0 0.0 0 0)
      (CallFunction|AnsweredCorrect)
      (else
        (Variables|Default|SetInput 0)
        (Variables|Default|SetAllCorrect 0)
        (Utilities|Array|Clear (Variables|Default|GetInputAnswer))
        (bind _output_get (Variables|Default|SetInputText ""))
        (Rendering|Components|TextRender|SetText (Variables|Default|GetAnswer) (Utilities|Text|ToText(String) _output_get))
        (Audio|PlaySound2D "/Game/Audio/mixkit-system-beep-buzzer-fail-2964.mixkit-system-beep-buzzer-fail-2964" 1.0 1.0 0.0 0 0)))))

(event Custom|AnsweredCorrect
  (for _array_element (Variables|Default|GetDoor)
    (Actor|DestroyActor _array_element))
  (bind _foundwidgets (Widget|GetAllWidgetsOfClass "/Game/UI/WB_TabeMenu.WB_TabeMenu_C" true))
  (Default|ObjectiveComplete _foundwidgets (Variables|Default|GetObjectiveCheck)))

(event EventBeginPlay
  (bind _returnvalue (Actor|GetActorOfClass "/Game/Blueprints/BP_RandomNumberParent.BP_RandomNumberParent_C"))
  (Variables|Default|SetActAnswer (Variables|/Game/Blueprints/BP_RandomNumberParent.BP_RandomNumberParent_C|GetNumberArray _returnvalue)))

(fn ConstructionScript)