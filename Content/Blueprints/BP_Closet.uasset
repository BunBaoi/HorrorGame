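; Closet hiding spot that lets the first-person player hide inside and step back out with the interact input.
; Box overlap gates the input; interacting toggles the character's visibility and collision and blends the view between closet and player.
; Each interaction also replays a timeline that swings both doors between closed and open angles.
; A short delay after toggling re-enables input and reopens the gate.
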(event OnComponentBeginOverlap(Box)
  (params (OverlappedComponent :type Primitive%20Component%20Object%20Reference) (OtherActor :type Actor%20Object%20Reference) (OtherComp :type Primitive%20Component%20Object%20Reference) (OtherBodyIndex :type Integer) (bFromSweep :type Boolean) (SweepResult :type Hit%20Result%20Structure%20%28by%20ref%29))
  (bind _asbp_first_person_character (Utilities|Casting|CastToBP_FirstPersonCharacter OtherActor))
  (Variables|Default|SetChar%20Ref _asbp_first_person_character)
  (Input|EnableInput (Game|GetPlayerController 0))
  (Utilities|FlowControl|Gate true) ; enters at Open
)

(event OnComponentEndOverlap(Box)
  (params (OverlappedComponent :type Primitive%20Component%20Object%20Reference) (OtherActor :type Actor%20Object%20Reference) (OtherComp :type Primitive%20Component%20Object%20Reference) (OtherBodyIndex :type Integer))
  (bind _returnvalue (Game|GetPlayerController 0))
  (Utilities|Casting|CastToBP_FirstPersonCharacter OtherActor)
  (Input|DisableInput _returnvalue 0)
  (Utilities|FlowControl|Gate true) ; enters at Close
)

(event Input|EnhancedActionEvents|EnhancedInputActionIA_Interact
  (params (ActionValue :type Boolean) (ElapsedSeconds :type Float%20%28double-precision%29) (TriggeredSeconds :type Float%20%28double-precision%29) (InputAction :type Input%20Action%20Object%20Reference :default "/Game/FirstPerson/Input/Actions/IA_Interact.IA_Interact"))
  (:Started
    (Utilities|FlowControl|Gate true :!label _label
      (:Exit
        (Utilities|FlowControl|Sequence
          (:then_0
            (CallFunction|ToggleHide)
            (Utilities|FlowControl|Delay 0.2)
            (Input|EnableInput (Game|GetPlayerController 0))
            (goto _label Open))
          (:then_1
            (|OpenCloseDoor)))))))

(fn ConstructionScript)

(fn ToggleHide
  (bind _returnvalue (Game|GetPlayerController 0))
  (bind _char_ref (Variables|Default|GetChar%20Ref))
  (if (Variables|Default|GetIsHiding?)
    (Variables|Default|SetIsHiding? false)
    (Rendering|SetActorHiddenInGame _char_ref false)
    (Collision|SetActorEnableCollision _char_ref true)
    (Game|Player|SetViewTargetwithBlend _returnvalue _char_ref 1.0 "VTBlend_Linear" 0.0 false)
    (else
      (Variables|Default|SetIsHiding? true)
      (Rendering|SetActorHiddenInGame _char_ref true)
      (Collision|SetActorEnableCollision _char_ref false)
      (Game|Player|SetViewTargetwithBlend _returnvalue self 1.0 "VTBlend_Linear" 0.0 false))))