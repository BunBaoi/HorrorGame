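; TempSprint is a Blueprint that prototypes stamina-limited sprinting on a character's movement component.
; Pressing Sprint raises walk speed and drains stamina in a half-second Delay loop until release or depletion.
; Stopping sets walk speed to zero and starts a matching recovery loop, though its increment is zero, so stamina never refills.
; Each stamina step fires the OnStaminaUsed dispatcher through UpdateStamina.
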(event Custom|UpdateStamina
  (Default|CallOnStaminaUsed))

(event Input|ActionEvents|InputActionSprint
  (params (Key :type Key%20Structure :default "None"))
  (bind _charactermovement (Variables|Character|GetCharacterMovement))
  (:Pressed
    (if (not (Variables|Default|GetIs%20Running?))
      (if (> (Variables|Default|GetStamina) 0.0) :!label _label
        (Variables|Default|SetIs%20Running? true)
        (Variables|/Script/Engine.CharacterMovementComponent|SetMaxWalkSpeed _charactermovement 5e+02)
        (Variables|Default|SetStamina (Math|Float|Clamp(Float) (- (Variables|Default|GetStamina) 0.5) 0.0 (Variables|Default|GetMaxStamina)))
        (CallFunction|UpdateStamina)
        (Utilities|FlowControl|Delay 0.5)
        (if (Variables|Default|GetIs%20Running?)
          (goto _label))
        (else
          (Variables|/Script/Engine.CharacterMovementComponent|SetMaxWalkSpeed _charactermovement 0.0 :!label _label_2)
          (Variables|Default|SetIs%20Running? false)
          (if (not (== (Variables|Default|GetMaxStamina) (Variables|Default|GetStamina))) :!label _label_3
            (Variables|Default|SetStamina (Math|Float|Clamp(Float) (+ (Variables|Default|GetStamina) 0.0) 0.0 (Variables|Default|GetMaxStamina)))
            (CallFunction|UpdateStamina)
            (Utilities|FlowControl|Delay 0.5)
            (if (not (Variables|Default|GetIs%20Running?))
              (goto _label_3)))))))
  (:Released
    (goto _label_2)))

(fn ConstructionScript)