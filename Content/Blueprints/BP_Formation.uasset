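; BP_Formation is a formation anchor that follows BP_FirstPersonCharacter and pulls BP_Entity actors toward five position components.
; BeginPlay caches all entities, and each Tick sets the anchor from the character's X/Y location and roll/pitch, without its Z or yaw.
; Tick also plays a timeline that lerps each entity from its current location to the slot matching its array index, without sweeping or a bounds check.
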(event EventTick
  (params (DeltaSeconds :type Float%20%28single-precision%29))
  (bind _entityarray (Variables|Default|GetEntityArray))
  (Utilities|FlowControl|Sequence
    (:then_0
      (bind _returnvalue (Actor|GetActorOfClass "/Game/FirstPerson/Blueprints/BP_FirstPersonCharacter.BP_FirstPersonCharacter_C"))
      (Transformation|SetActorLocation (Math|Vector|MakeVector (.x (Transformation|GetActorLocation _returnvalue)) (.y (Transformation|GetActorLocation _returnvalue)) 0.0) false false)
      (Transformation|SetActorRotation (Math|Rotator|MakeRotator (.roll (Transformation|GetActorRotation _returnvalue)) (.pitch (Transformation|GetActorRotation _returnvalue)) 0.0)))
    (:then_1
      ;[1 1 1] Loop for ai to move to location with timeline as movement
      (Variables|Default|SetPositionLocations (Utilities|Array|MakeArray (Transformation|GetWorldLocation (Variables|Default|GetPosition1)) (Transformation|GetWorldLocation (Variables|Default|GetPosition2)) (Transformation|GetWorldLocation (Variables|Default|GetPosition3)) (Transformation|GetWorldLocation (Variables|Default|GetPosition4)) (Transformation|GetWorldLocation (Variables|Default|GetPosition5))))
      (bind _formationfloat (Timeline|Timeline Play)
        (:Update
          (for (_array_element _array_index) _entityarray
            (Transformation|SetActorLocation _array_element (Math|Vector|Lerp(Vector) (Transformation|GetActorLocation (Utilities|Array|Get(acopy) _entityarray _array_index)) (Utilities|Array|Get(acopy) (Variables|Default|GetPositionLocations) _array_index) _formationfloat) false false)))))))

(event EventBeginPlay
  (bind _outactors (Actor|GetAllActorsOfClass "/Game/Blueprints/BP_Entity.BP_Entity_C"))
  (Variables|Default|SetEntityArray _outactors))

(fn ConstructionScript)