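; BP_Summoning-Circle is a candle-order puzzle that numbers its child BP_Candle actors from one on BeginPlay.
; CandleCheck compares an incoming number with AnswerArray at the current step, lighting the candle at that array position and advancing on a match.
; A mismatch resets progress and puts out every candle.
; The completion branch is empty, and CheckCandle, which increments the player's CandleIndex, looks unfinished with a self-comparing condition.
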(event Custom|LightCandleCase)

(event Custom|CandleCheck
  (params (InputInt :type Integer))
  (Development|PrintString (Utilities|String|ToString(Integer) InputInt))
  (if (== InputInt (Utilities|Array|Get(acopy) (Variables|Default|GetAnswerArray) (Variables|Default|GetCheckinc)))
    (bind _asbp_candle (Utilities|Casting|CastToBP_Candle (Utilities|Array|Get(acopy) (Variables|Default|GetCandleLitArray) (Variables|Default|GetCheckinc))))
    (Default|LightCandle _asbp_candle)
    (Math|Integer|IncrementInt (Variables|Default|GetCheckinc)
      (:%20%20
        (if (== (Variables|Default|GetCheckinc) (Variables|Default|GetCheckinc))
          _)))
    (else
      (for _array_element (Variables|Default|GetCandleLitArray)
        (Variables|Default|SetCheckinc 0)
        (bind _asbp_candle_2 (Utilities|Casting|CastToBP_Candle _array_element))
        (Default|CandleOut _asbp_candle_2)))))

(event EventBeginPlay
  (bind _output_get (Variables|Default|SetCandleLitArray (Actor|GetAllChildActors false)))
  (for (_array_element _array_index) _output_get
    (bind _asbp_candle (Utilities|Casting|CastToBP_Candle _array_element))
    (Variables|/Game/Blueprints/BP_Candle.BP_Candle_C|SetNum _asbp_candle (+ _array_index 1))))

(fn ConstructionScript)

(fn CheckCandle
  (bind _c1 (Variables|Default|GetC1))
  (bind _returnvalue (Actor|GetActorOfClass "/Game/FirstPerson/Blueprints/BP_FirstPersonCharacter.BP_FirstPersonCharacter_C"))
  (if (== (Variables|/Game/FirstPerson/Blueprints/BP_FirstPersonCharacter.BP_FirstPersonCharacter_C|GetCandleIndex _returnvalue) (Variables|/Game/FirstPerson/Blueprints/BP_FirstPersonCharacter.BP_FirstPersonCharacter_C|GetCandleIndex _returnvalue))
    (Math|Integer|IncrementInt (Variables|/Game/FirstPerson/Blueprints/BP_FirstPersonCharacter.BP_FirstPersonCharacter_C|GetCandleIndex _returnvalue)
      (:%20%20
        (ChildActorComponent|SetChildActorClass _c1 (Variables|/Script/Engine.ChildActorComponent|GetChildActorClass _c1))))))