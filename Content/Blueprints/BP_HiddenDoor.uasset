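; BP_HiddenDoor is a secret door that opens alongside a rotating book when OpenDoor is called.
; A Timeline with separate tracks tilts the book's pitch and swings the door's yaw between set angles.
; Every Timeline update also looks up WB_TabeMenu widgets and calls ObjectiveComplete on them with ObjectiveCheck.
; A DoOnce blocks retriggering until the Timeline finishes, and no closing logic exists.
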(event Custom|OpenDoor
  (Utilities|FlowControl|DoOnce false :!label _label
    (:Completed
      (bind (_direction _booktrack _doortrack) (Timeline|Timeline Play)
        (:Update
          (Transformation|SetRelativeRotation (Variables|Default|Getbook) (Math|Rotator|MakeRotator 0.0 (Math|Float|Lerp (Variables|Default|GetBookin) (Variables|Default|GetBookOut) _booktrack) -9e+01) false false)
          (Transformation|SetRelativeRotation (Variables|Default|GetDoor) (Math|Rotator|MakeRotator 0.0 0.0 (Math|Float|Lerp (Variables|Default|GetDoorClosed) (Variables|Default|GetDoorOpen) _doortrack)) false false)
          (bind _foundwidgets (Widget|GetAllWidgetsOfClass "/Game/UI/WB_TabeMenu.WB_TabeMenu_C" true))
          (Default|ObjectiveComplete _foundwidgets (Variables|Default|GetObjectiveCheck)))
        (:Finished
          (goto _label Reset))))))

(fn ConstructionScript)