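; Door actor Blueprint that swings open and closed and shows a widget while something is near it.
; A sphere's begin and end overlap events toggle the widget's visibility.
; The OpenDoor event uses a FlipFlop to alternately play a timeline from the start or reverse it.
; The timeline's float lerps the door mesh's relative yaw between closed and opened angles.
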(event OnComponentBeginOverlap(Sphere)
  (params (OverlappedComponent :type Primitive%20Component%20Object%20Reference) (OtherActor :type Actor%20Object%20Reference) (OtherComp :type Primitive%20Component%20Object%20Reference) (OtherBodyIndex :type Integer) (bFromSweep :type Boolean) (SweepResult :type Hit%20Result%20Structure%20%28by%20ref%29))
  (Rendering|SetVisibility (Variables|Default|GetWidget) true false))

(event OnComponentEndOverlap(Sphere)
  (params (OverlappedComponent :type Primitive%20Component%20Object%20Reference) (OtherActor :type Actor%20Object%20Reference) (OtherComp :type Primitive%20Component%20Object%20Reference) (OtherBodyIndex :type Integer))
  (Rendering|SetVisibility (Variables|Default|GetWidget) false false))

(event Custom|OpenDoor
  (Utilities|FlowControl|FlipFlop
    (:A
      (bind _doorfloat (Timeline|OpenDoor%20TimeLine PlayFromStart)
        (:Update
          (Transformation|SetRelativeRotation (Variables|Default|GetSM_Door_1A_Submesh_0CE543D7) (Math|Rotator|MakeRotator 0.0 0.0 (Math|Float|Lerp (Variables|Default|GetDoorClosed) (Variables|Default|GetDoorOpened) _doorfloat)) false false))))
    (:B
      (Timeline|OpenDoor%20TimeLine Reverse))))

(fn ConstructionScript)