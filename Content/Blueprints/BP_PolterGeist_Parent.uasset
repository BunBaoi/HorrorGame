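; BP_PolterGeist_Parent is a poltergeist actor that shakes its Chair component with random physics forces, toggled by Move and StopMove events.
; While active, Tick waits random delays, rolls against MoveChance, then picks a random force direction, magnitude and application point within the inner actor bounds.
; A second gate applies that force every frame until a random duration delay closes it.
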(event Custom|Move
  (bind (_origin _boxextent) (Collision|GetActorBounds false false))
  (Utilities|FlowControl|Gate true) ; enters at Open
)

(event Custom|StopMove
  (bind (_origin _boxextent) (Collision|GetActorBounds false false))
  (Utilities|FlowControl|Gate true) ; enters at Close
)

(event EventBeginPlay)

(event Collision|EventActorBeginOverlap
  (params (OtherActor :type Actor%20Object%20Reference)))

(event EventTick
  (params (DeltaSeconds :type Float%20%28single-precision%29))
  (bind (_origin _boxextent) (Collision|GetActorBounds false false))
  (Utilities|FlowControl|Gate true
    (:Exit
      (Utilities|FlowControl|Sequence
        (:then_0
          (Utilities|FlowControl|Gate true :!label _label
            (:Exit
              (Class|PrimitiveComponent|AddForceatLocation (Variables|Default|GetChair) (Variables|Default|GetMoveForce) (Variables|Default|GetForce%20Loc) "None"))))
        (:then_1
          (Utilities|FlowControl|Delay (Math|Random|RandomFloatinRange 0.0 (Variables|Default|GetMaxMoveDelay)))
          (if (>= (Math|Random|RandomFloatinRange 0.0 1e+02) (Variables|Default|GetMoveChance))
            (Utilities|FlowControl|Sequence
              (:then_0
                (Variables|Default|SetMoveForce (* (Math|Random|RandomUnitVector) (Math|Random|RandomFloatinRange (Variables|Default|GetMiniMoveForce) (Variables|Default|GetMaxMoveForce))))
                (Variables|Default|SetForce%20Loc (Math|Random|RandomPointinBoundingBox _origin (/ _boxextent 2.0)))
                (goto _label Open))
              (:then_1
                (Utilities|FlowControl|Delay (Math|Random|RandomFloatinRange 0.0 (Variables|Default|GetMaxForceDuration)))
                (goto _label Close)))))))))

(fn ConstructionScript)