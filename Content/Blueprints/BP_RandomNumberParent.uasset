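; BP_RandomNumberParent shows random digits on placed text actors that are only visible while the player's flashlight is off.
; On BeginPlay it fills NumberArray with one random 1–9 value per NumberActorArray entry, then writes each to the matching TextRenderActor.
; Every Tick it polls the flashlight flag on BP_FirstPersonCharacter and hides or shows all the number actors accordingly.
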(event EventBeginPlay
  (Utilities|FlowControl|Sequence
    (:then_0
      (Utilities|Array|Clear (Variables|Default|GetNumberArray))
      (for (_ _array_index) (Variables|Default|GetNumberActorArray)
        (Utilities|Array|Add (Variables|Default|GetNumberArray) _array_index))
      (for (_ _array_index_2) (Variables|Default|GetNumberArray)
        (Utilities|Array|SetArrayElem (Variables|Default|GetNumberArray) _array_index_2 (Math|Random|RandomIntegerinRange 1 9))))
    (:then_1
      (for (_array_element _array_index_3) (Variables|Default|GetNumberActorArray)
        (bind _astext_render_actor (Utilities|Casting|CastToTextRenderActor _array_element))
        (Rendering|Components|TextRender|SetText (Variables|/Script/Engine.TextRenderActor|GetTextRender _astext_render_actor) (Utilities|Text|ToText(Integer) (Utilities|Array|Get(acopy) (Variables|Default|GetNumberArray) _array_index_3)))))))

(event Collision|EventActorBeginOverlap
  (params (OtherActor :type Actor%20Object%20Reference)))

(event EventTick
  (params (DeltaSeconds :type Float%20%28single-precision%29))
  (bind _asbp_first_person_character (Utilities|Casting|CastToBP_FirstPersonCharacter (Game|GetPlayerCharacter 0)))
  (if (Variables|/Game/FirstPerson/Blueprints/BP_FirstPersonCharacter.BP_FirstPersonCharacter_C|Getflaslight%20Active _asbp_first_person_character)
    (for (_ _array_index) (Variables|Default|GetNumberActorArray)
      (Rendering|SetActorHiddenInGame (Utilities|Array|Get(acopy) (Variables|Default|GetNumberActorArray) _array_index) true))
    (else
      (for (_ _array_index_2) (Variables|Default|GetNumberActorArray)
        (Rendering|SetActorHiddenInGame (Utilities|Array|Get(acopy) (Variables|Default|GetNumberActorArray) _array_index_2) false)))))

(fn ConstructionScript)