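; BP_anchor is a roaming character that acts as the shared anchor for a group of BP_Entity rats.
; It gathers every BP_Entity at BeginPlay, then loops through AI moves to random nearby reachable points, telling them to Run when moving and Idle on arrival.
; End calls Runaway on each rat and destroys the anchor.
; Helper functions adjust walk speed (StartSprint zeroes it) and play trace-checked footstep sounds.
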(event Custom|Roam
  (if (not (Variables|Default|GetRunaway))
    (AI|AIMoveTo self (.RandomLocation (AI|Navigation|GetRandomReachablePointinRadius (Transformation|GetActorLocation) 5e+02 0 0)) 0 5.0 false
      (:then
        (for _array_element (Variables|Default|GetRatsArray)
          (bind _asbp_entity (Utilities|Casting|CastToBP_Entity _array_element))
          (Default|Run _asbp_entity)))
      (:OnSuccess
        (for _array_element_2 (Variables|Default|GetRatsArray)
          (bind _asbp_entity_2 (Utilities|Casting|CastToBP_Entity _array_element_2))
          (Default|Idle _asbp_entity_2))
        (Utilities|FlowControl|Delay 1e+01)
        (CallFunction|Roam)))))

(event Custom|End
  (Variables|Default|SetRunaway false)
  (for _array_element (Variables|Default|GetRatsArray)
    (bind _asbp_entity (Utilities|Casting|CastToBP_Entity _array_element))
    (Default|Runaway _asbp_entity))
  (Actor|DestroyActor))

(event EventBeginPlay
  (Utilities|FlowControl|Sequence
    (:then_0
      (bind _outactors (Actor|GetAllActorsOfClass "/Game/Blueprints/FormationBPs/BP_Entity.BP_Entity_C"))
      (Variables|Default|SetRatsArray _outactors))
    (:then_1
      (Variables|/Script/Engine.CharacterMovementComponent|SetMaxWalkSpeed (Variables|Character|GetCharacterMovement) (Variables|Default|GetWalkSpeed))
      (CallFunction|Roam))))

(fn ConstructionScript)

(fn StartSprint
  (Variables|/Script/Engine.CharacterMovementComponent|SetMaxWalkSpeed (Variables|Character|GetCharacterMovement) 0.0))

(fn StopSprint
  (Variables|/Script/Engine.CharacterMovementComponent|SetMaxWalkSpeed (Variables|Character|GetCharacterMovement) (Variables|Default|GetWalkSpeed)))

(fn TraceFootsteps
  (bind _returnvalue (Transformation|GetActorLocation))
  (bind _capsulecomponent (Variables|Collision|GetCapsuleComponent))
  (bind (_x _y _z) (Math|Vector|BreakVector _returnvalue))
  (bind _returnvalue_2 (Collision|SphereTraceByChannel _returnvalue (Math|Vector|MakeVector _x _y (- _z (Components|Capsule|GetScaledCapsuleHalfHeight _capsulecomponent))) (Components|Capsule|GetScaledCapsuleRadius _capsulecomponent) "TraceTypeQuery1" false 0 "None"))
  (return _returnvalue_2))

(fn FootstepTry
  (bind _finished (CallFunction|TraceFootsteps))
  (if _finished
    (Audio|PlaySoundatLocation 0 (Transformation|GetActorLocation) "0, 0, 0" 1.0 1.0 0.0 0 0 0 0)))