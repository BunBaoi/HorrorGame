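; Ghost spirit AI that wanders the level and sways nearby ceiling lights as it passes.
; On BeginPlay it spawns an AIController and starts roaming to random reachable points, choosing a new one after each successful move.
; A Box overlap tracks actors tagged "Sway", and Tick pushes each tracked ceiling light with a force scaled by its distance from the ghost.
; Point light intensity and color nodes are present but never run.
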(event OnComponentBeginOverlap(Box)
  (params (OverlappedComponent :type Primitive%20Component%20Object%20Reference) (OtherActor :type Actor%20Object%20Reference) (OtherComp :type Primitive%20Component%20Object%20Reference) (OtherBodyIndex :type Integer) (bFromSweep :type Boolean) (SweepResult :type Hit%20Result%20Structure%20%28by%20ref%29))
  (if (Actor|ActorHasTag OtherActor "Sway")
    (Utilities|Array|Add (Variables|Default|GetMoveLightsArray) OtherActor)))

(event OnComponentEndOverlap(Box)
  (params (OverlappedComponent :type Primitive%20Component%20Object%20Reference) (OtherActor :type Actor%20Object%20Reference) (OtherComp :type Primitive%20Component%20Object%20Reference) (OtherBodyIndex :type Integer))
  (Utilities|Array|RemoveItem (Variables|Default|GetMoveLightsArray) OtherActor))

(event Custom|Random%20Roam
  (AI|AIMoveTo self (.RandomLocation (AI|Navigation|GetRandomReachablePointinRadius (Transformation|GetActorLocation) 2.5e+03 0 0)) 0 5.0 false
    (:OnSuccess
      (CallFunction|RandomRoam))))

(event EventTick
  (params (DeltaSeconds :type Float%20%28single-precision%29))
  (for _array_element (Variables|Default|GetMoveLightsArray)
    (bind _asblueprint_ceiling_light (Utilities|Casting|CastToBlueprint_CeilingLight _array_element))
    (Class|PrimitiveComponent|AddForceatLocation (Variables|/Game/Blueprints/Blueprint_CeilingLight.Blueprint_CeilingLight_C|GetCombined_9D578029 _asblueprint_ceiling_light) (Math|Vector|MakeVector (.x (* 0.05 (Transformation|GetDistanceTo _asblueprint_ceiling_light self))) (.y (* 0.05 (Transformation|GetDistanceTo _asblueprint_ceiling_light self))) 0.0) "0, 0, 0" "None")))

(event EventBeginPlay
  (Game|SpawnActorfromClass "/Script/AIModule.AIController" (Math|Conversions|ToTransform(Vector) (Transformation|GetActorLocation)) "Undefined" "MultiplyWithRoot" 0 0)
  (CallFunction|RandomRoam)
  (Development|PrintString "playing"))

(fn ConstructionScript)