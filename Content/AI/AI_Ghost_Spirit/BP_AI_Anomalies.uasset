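; BP_AI_Anomalies is an AI anomaly character that homes in on the player.
; Tick calls Moveto, which plays a timeline that lerps the actor from its current location toward player 0, using SetActorLocation without sweep.
; UpdateSpeed sets the CharacterMovement max walk speed, which that direct movement does not use.
; The AI perception events are empty stubs.
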(event OnComponentActivated(AIPerception)
  (params (Component :type Actor%20Component%20Object%20Reference) (bReset :type Boolean)))

(event OnTargetPerceptionUpdated(AIPerception)
  (params (Actor :type Actor%20Object%20Reference) (Stimulus :type AI%20Stimulus%20Structure)))

(event Custom|Moveto
  (bind _floatmove (Timeline|Timeline Play)
    (:Update
      (Transformation|SetActorLocation (Math|Vector|Lerp(Vector) (Transformation|GetActorLocation) (Transformation|GetActorLocation (Game|GetPlayerCharacter 0)) _floatmove) false false))))

(event EventTick
  (params (DeltaSeconds :type Float%20%28single-precision%29))
  (CallFunction|Moveto))

(fn ConstructionScript)

(fn UpdateSpeed
  (params (UpdateSpeed :type Float%20%28double-precision%29))
  (Variables|/Script/Engine.CharacterMovementComponent|SetMaxWalkSpeed (Variables|Character|GetCharacterMovement) UpdateSpeed))