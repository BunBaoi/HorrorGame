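; Ghost spirit anomaly AI that glides at the player and vanishes on contact.
; When Moveto fires, a timeline repeatedly lerps it from its current location toward the player's live position without sweep, ignoring obstacles, with a one-time running sound.
; Overlapping the first-person character destroys it and plays a creepy child laugh.
; A helper sets walk speed, though the timeline motion bypasses character movement.
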(event OnComponentBeginOverlap(Collision)
  (params (OverlappedComponent :type Primitive%20Component%20Object%20Reference) (OtherActor :type Actor%20Object%20Reference) (OtherComp :type Primitive%20Component%20Object%20Reference) (OtherBodyIndex :type Integer) (bFromSweep :type Boolean) (SweepResult :type Hit%20Result%20Structure%20%28by%20ref%29))
  (Utilities|Casting|CastToBP_FirstPersonCharacter OtherActor)
  (Actor|DestroyActor)
  (Audio|PlaySound2D "/Game/Audio/SW_Creep_Kid_Laugh.SW_Creep_Kid_Laugh" 1.0 1.0 0.0 0 0))

(event Custom|Moveto
  (params (Object :type Actor%20Object%20Reference))
  (bind _floatmove (Timeline|Timeline Play)
    (:Update
      (Transformation|SetActorLocation (Math|Vector|Lerp(Vector) (Transformation|GetActorLocation) (Transformation|GetActorLocation (Game|GetPlayerCharacter 0)) _floatmove) false false)
      (Utilities|FlowControl|DoOnce false
        (:Completed
          (Audio|PlaySoundatLocation "/Game/Audio/SW_Running.SW_Running" (Math|Vector|Lerp(Vector) (Transformation|GetActorLocation) (Transformation|GetActorLocation (Game|GetPlayerCharacter 0)) _floatmove) "0, 0, 0" 1.0 1.0 0.0 0 0 0 0))))))

(fn ConstructionScript)

(fn UpdateSpeed
  (params (UpdateSpeed :type Float%20%28double-precision%29))
  (Variables|/Script/Engine.CharacterMovementComponent|SetMaxWalkSpeed (Variables|Character|GetCharacterMovement) UpdateSpeed))