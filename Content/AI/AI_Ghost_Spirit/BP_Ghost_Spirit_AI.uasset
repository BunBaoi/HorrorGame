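; Ghost spirit AI that continually flees from the player and makes nearby ceiling lights sway.
; From BeginPlay, RunAway repeatedly issues AI moves to a point a short step directly away from the player, retrying on success or failure.
; An overlap sphere tracks actors tagged "Sway", and Tick pushes those ceiling lights with a distance-scaled force.
; A self-repeating RandomRoam event exists but nothing here calls it.
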(event OnComponentBeginOverlap(Sphere)
  (params (OverlappedComponent :type Primitive%20Component%20Object%20Reference) (OtherActor :type Actor%20Object%20Reference) (OtherComp :type Primitive%20Component%20Object%20Reference) (OtherBodyIndex :type Integer) (bFromSweep :type Boolean) (SweepResult :type Hit%20Result%20Structure%20%28by%20ref%29))
  ;[1 1 1] AI Interact Lights
  (if (Actor|ActorHasTag OtherActor "Sway")
    (Utilities|Array|Add (Variables|Default|GetMoveLightsArray) OtherActor)))

(event OnComponentEndOverlap(Sphere)
  (params (OverlappedComponent :type Primitive%20Component%20Object%20Reference) (OtherActor :type Actor%20Object%20Reference) (OtherComp :type Primitive%20Component%20Object%20Reference) (OtherBodyIndex :type Integer))
  ;[1 1 1] AI Interact Lights
  (Utilities|Array|RemoveItem (Variables|Default|GetMoveLightsArray) OtherActor))

(event Custom|Run%20Away
  (bind _returnvalue (Transformation|GetActorLocation))
  (bind _char_ref (Variables|Default|GetChar%20Ref))
  (bind _returnvalue_2 (Transformation|GetActorLocation _char_ref))
  (bind _returnvalue_3 (Math|Rotator|FindLookatRotation _returnvalue _returnvalue_2))
  (bind _returnvalue_4 (Math|Vector|GetForwardVector _returnvalue_3))
  (bind _returnvalue_5 (* _returnvalue_4 -6e+01))
  (bind _returnvalue_6 (+ _returnvalue _returnvalue_5))
  (bind (_x _y) (Math|Vector|BreakVector _returnvalue_6))
  ;[1 1 1] AI Status - Run Away
  ;;[1 1 1] Acceptance Radius = Detection raduis
  (AI|AIMoveTo self (Math|Vector|MakeVector _x _y (.Z (Math|Vector|BreakVector _returnvalue))) 0 5e+01 false
    (:OnSuccess
      _)
    (:OnFail
      _))
  (CallFunction|RunAway))

(event Custom|Random%20Roam
  ;[1 1 1] AI Status - Roam
  (AI|AIMoveTo self (.RandomLocation (AI|Navigation|GetRandomReachablePointinRadius (Transformation|GetActorLocation) 2.5e+03 0 0)) 0 5.0 false
    (:OnSuccess
      (CallFunction|RandomRoam))))

(event EventTick
  (params (DeltaSeconds :type Float%20%28single-precision%29))
  ;[1 1 1] AI Interact Lights
  (for _array_element (Variables|Default|GetMoveLightsArray)
    (bind _asblueprint_ceiling_light (Utilities|Casting|CastToBlueprint_CeilingLight _array_element))
    (Class|PrimitiveComponent|AddForceatLocation (Variables|/Game/Blueprints/Blueprint_CeilingLight.Blueprint_CeilingLight_C|GetCombined_9D578029 _asblueprint_ceiling_light) (Math|Vector|MakeVector (.x (* 0.05 (Transformation|GetDistanceTo _asblueprint_ceiling_light self))) (.y (* 0.05 (Transformation|GetDistanceTo _asblueprint_ceiling_light self))) 0.0) "0, 0, 0" "None")))

(event EventBeginPlay
  ;[1 1 1] AI Status - Run Away
  (bind _asbp_first_person_character (Utilities|Casting|CastToBP_FirstPersonCharacter (Game|GetPlayerCharacter 0)))
  (Variables|Default|SetChar%20Ref _asbp_first_person_character)
  (CallFunction|RunAway))

(fn ConstructionScript)