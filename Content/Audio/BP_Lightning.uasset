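; BP_Lightning is an actor that plays recurring thunder sounds in the level; no visual flash is scripted.
; At BeginPlay, each instance collects all BP_Lightning actors as candidate sound locations.
; A Tick-driven DoOnce plays its ThunderCUe and a thunder cue at a random instance's location, then resets after a random delay, so every placed instance runs its own loop.
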(event EventBeginPlay
  (bind _outactors (Actor|GetAllActorsOfClass "BP_Lightning_C"))
  (Variables|Default|SetLocationsArray _outactors))

(event Collision|EventActorBeginOverlap
  (params (OtherActor :type Actor%20Object%20Reference)))

(event EventTick
  (params (DeltaSeconds :type Float%20%28single-precision%29))
  (Utilities|FlowControl|DoOnce false :!label _label
    (:Completed
      (Audio|Components|Audio|Play (Variables|Default|GetThunder_CUe) 0.0)
      (Audio|PlaySoundatLocation "/Game/Audio/Thunder_CUe.Thunder_CUe" (Transformation|GetActorLocation (.OutItem (Utilities|Array|Random (Variables|Default|GetLocationsArray)))) "0, 0, 0" 1.0 1.0 0.0 0 0 0 0)
      (Utilities|FlowControl|Delay (Math|Random|RandomFloatinRange 45.0 1e+02))
      (goto _label Reset))))

(fn ConstructionScript)